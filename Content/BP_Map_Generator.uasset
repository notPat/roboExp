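; Map generator actor that runs a timed multi-robot exploration, collecting lidar scans into a point cloud.
; On BeginPlay it spawns waypoints at navmesh-reachable grid points and color-coded BP_AI robots, assigning waypoints by angular sector around itself.
; A looping timer gathers scanner points, while player controller signals toggle or rebuild the cloud render.
; When time expires or on signal, it exports the points as XYZ and opens the LidarCloud level.
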(event Custom|BuildMapSig_Event
  (for _array_element (Variables|Default|Getrobos)
    (Default|StorePoints (Variables|/Game/ProfectBPS/AI/BP_AI.BP_AI_C|GetScanner _array_element))
    (for _array_element_2 (Variables|/Game/ProfectBPS/LidarCloudGen/Scanner.Scanner_C|Getstored%20pos (Variables|/Game/ProfectBPS/AI/BP_AI.BP_AI_C|GetScanner _array_element))
      (Utilities|Array|Add (Variables|Default|GetLidar%20points) _array_element_2)))
  (Default|CallLidarRenderCloudSig (Variables|Default|GetLidar%20points))
  (Development|PrintString (Utilities|String|ToString(Integer) (Utilities|Array|Length (Variables|Default|GetLidar%20points)))))

(event Custom|ShowLidarSig_Event
  (bind _bp_lidar_point_cloud_renderer (Variables|Default|GetBP_Lidar_Point_Cloud_Renderer))
  (Utilities|FlowControl|FlipFlop
    (:A
      (Development|SetHiddeninGame _bp_lidar_point_cloud_renderer false false))
    (:B
      (Development|SetHiddeninGame _bp_lidar_point_cloud_renderer true false))))

(event Custom|RenderPointCloudInNewLevelSig_Event
  (bind _lidar_points (Variables|Default|GetLidar%20points))
  (for _array_element (Variables|Default|Getrobos)
    (Default|EndScanning (Variables|/Game/ProfectBPS/AI/BP_AI.BP_AI_C|GetScanner _array_element)))
  (Development|PrintString (Utilities|String|ToString(Integer) (Utilities|Array|Length _lidar_points)) true true "(R=0.000000,G=0.660000,B=1.000000,A=1.000000)" 3e+01)
  (CallFunction|BuildMapSigEvent)
  (Class|UtilityFunctions|ExportXYZ (Utilities|String|Append (Class|KismetSystemLibrary|GetProjectSavedDirectory) "Exports/tmp/" "tmp" ".xyz") _lidar_points 1.0)
  (Game|OpenLevel(byName) "LidarCloud" false))

(event Custom|store%20points%20in%20robots
  (for _array_element (Variables|Default|Getrobos)
    (Default|StorePoints (Variables|/Game/ProfectBPS/AI/BP_AI.BP_AI_C|GetScanner _array_element)))
  (for _array_element_2 (Variables|/Game/ProfectBPS/LidarCloudGen/Scanner.Scanner_C|Getstored%20pos (Variables|/Game/ProfectBPS/AI/BP_AI.BP_AI_C|GetScanner _array_element))
    (Utilities|Array|Add (Variables|Default|GetLidar%20points) _array_element_2))
  (Utilities|Array|Clear (Variables|/Game/ProfectBPS/LidarCloudGen/Scanner.Scanner_C|Getstored%20pos (Variables|/Game/ProfectBPS/AI/BP_AI.BP_AI_C|GetScanner _array_element))))

(event EventBeginPlay
  (bind _returnvalue (Game|GetPlayerController 0))
  (bind _returnvalue_2 (Transformation|GetActorLocation))
  (bind _returnvalue_3 (Transformation|GetActorLocation))
  (bind _waypoints (Variables|Default|GetWaypoints))
  (bind (_projectedlocation _returnvalue_4) (AI|Navigation|ProjectPointtoNavigation _returnvalue_3 0 0 "200.000000,200.000000,1000.000000"))
  (Variables|/Script/Engine.PlayerController|SetbShowMouseCursor _returnvalue false)
  (Input|SetInputModeGameOnly _returnvalue false)
  (bind _asbp_explore_instance (Utilities|Casting|CastToBP_ExploreInstance (Game|GetGameInstance)))
  (Variables|Default|SetExploration%20Time (Variables|/Game/ProfectBPS/BP_ExploreInstance.BP_ExploreInstance_C|GetExplorationTime _asbp_explore_instance))
  (Variables|Default|SetroboAmount (- (Variables|/Game/ProfectBPS/BP_ExploreInstance.BP_ExploreInstance_C|GetRobotAmount _asbp_explore_instance) 1))
  (bind _returnvalue_5 (Class|UtilityFunctions|GenGridArray _returnvalue_2 (Variables|Default|GetmaxX) (Variables|Default|GetminX) (Variables|Default|GetmaxY) (Variables|Default|GetminY) (Variables|Default|GetmaxZ) (Variables|Default|GetminZ) 1000))
  (for _array_element _returnvalue_5
    (bind _returnvalue_6 (Class|NavigationSystemV1|FindPathtoLocationSynchronously _projectedlocation (.ProjectedLocation (AI|Navigation|ProjectPointtoNavigation _array_element 0 0 "200.000000,200.000000,1000.000000")) 0 0))
    (Variables|Default|SetWaypointNotThere true)
    (bind _array_element_2 (Utilities|Array|ForEachLoopwithBreak (Variables|Default|GetWaypoints) :!label _label)
      (:LoopBody
        (if (Utilities|Operators|EqualEqual (.ProjectedLocation (AI|Navigation|ProjectPointtoNavigation _array_element 0 0 "200.000000,200.000000,1000.000000")) (Transformation|GetActorLocation _array_element_2) 1e+01)
          (Variables|Default|SetWaypointNotThere false)
          (goto _label Break)))
      (:Completed
        (if (Math|Boolean|ANDBoolean (not (Class|NavigationPath|IsPartial _returnvalue_6)) _returnvalue_4 (.ReturnValue (AI|Navigation|ProjectPointtoNavigation _array_element 0 0 "200.000000,200.000000,1000.000000")) (Variables|Default|GetWaypointNotThere))
          (bind _returnvalue_7 (Game|SpawnActorfromClass "/Game/ProfectBPS/LidarCloudGen/BP_Waypoint.BP_Waypoint_C" (Math|Conversions|ToTransform(Vector) (+ (.ProjectedLocation (AI|Navigation|ProjectPointtoNavigation _array_element 0 0 "200.000000,200.000000,1000.000000")) "0.000000,0.000000,20.000000")) "Undefined" "MultiplyWithRoot" 0 0))
          (Variables|/Game/ProfectBPS/LidarCloudGen/BP_Waypoint.BP_Waypoint_C|SetSavedDistance _returnvalue_7 (Class|NavigationPath|GetPathLength _returnvalue_6))
          (Utilities|Array|AddUnique (Variables|Default|GetWaypoints) _returnvalue_7)))))
  (CallFunction|MakeColors)
  (for _index (range 0 (Variables|Default|GetroboAmount))
    (bind _newparam2 (CallFunction|MultVector _index _returnvalue_2))
    (bind _returnvalue_8 (Game|SpawnActorfromClass "/Game/ProfectBPS/AI/BP_AI.BP_AI_C" (Math|Conversions|ToTransform(Vector) (.ProjectedLocation (AI|Navigation|ProjectPointtoNavigation _newparam2 0 0 "200.000000,200.000000,500.000000"))) "AdjustIfPossibleButAlwaysSpawn" "MultiplyWithRoot" 0 0 0 0))
    (Variables|/Game/ProfectBPS/AI/BP_AI.BP_AI_C|SetSignitureColor _returnvalue_8 (Utilities|Array|Get(acopy) (Variables|Default|Getcolors) _index))
    (Utilities|Array|Insert (Variables|Default|Getrobos) _returnvalue_8))
  (for _array_element_3 _waypoints
    (if (== (Variables|/Game/ProfectBPS/LidarCloudGen/BP_Waypoint.BP_Waypoint_C|GetSavedDistance _array_element_3) -1.0)
      (Utilities|Array|Add (Variables|Default|GetWaypointFilter) _array_element_3)))
  (for _array_element_4 (Variables|Default|GetWaypointFilter)
    (Utilities|Array|RemoveItem _waypoints _array_element_4)
    (Actor|DestroyActor _array_element_4))
  (CallFunction|DistributePointstoRobots)
  (Utilities|Time|SetTimerbyFunctionName 0 "store points in robots" 1e+01 true)
  (bind _asbp_explore_player_controler (Utilities|Casting|CastToBP_ExplorePlayerControler (Game|GetPlayerController 0)))
  (EventDispatchers|AssignBuildMapSig _asbp_explore_player_controler (delegate Custom|BuildMapSig_Event))
  (EventDispatchers|AssignShowLidarSig _asbp_explore_player_controler (delegate Custom|ShowLidarSig_Event))
  (EventDispatchers|AssignRenderPointCloudinNewLevelSig _asbp_explore_player_controler (delegate Custom|RenderPointCloudInNewLevelSig_Event))
  (Utilities|Time|SetTimerbyFunctionName 0 "RenderPointCloudInNewLevelSig_Event" (Variables|Default|GetExploration%20Time))
  (for _array_element_5 (Variables|Default|Getrobos)
    (Default|StartUp _array_element_5)))

(fn ConstructionScript)

(fn MultVector
  (params (NewParam :type Integer) (NewParam1 :type Vector))
  (return (+ NewParam1 (* (Math|Conversions|ToVector(Float) NewParam) "-400.000000,0.000000,0.000000"))))

(fn DistributePointstoRobots
  (bind _returnvalue (Transformation|GetActorLocation))
  (bind _robos (Variables|Default|Getrobos))
  (bind _returnvalue_2 (Utilities|Array|Length _robos))
  (bind (_x _y) (Math|Vector|BreakVector _returnvalue))
  (bind _returnvalue_3 (- _returnvalue_2 0))
  (for _array_element (Variables|Default|GetWaypoints)
    (if (>= _x (.Y (Math|Vector|BreakVector (Transformation|GetActorLocation _array_element))))
      (Variables|Default|SetdividerTempVar (- 3.6e+02 (Class|KismetMathLibrary|DegAcos (Math|Vector|DotProduct (Variables|Default|GetXvector) (Math|Vector|Normalize (- (Math|Vector|MakeVector (.X (Math|Vector|BreakVector (Transformation|GetActorLocation _array_element))) (.Y (Math|Vector|BreakVector (Transformation|GetActorLocation _array_element))) 0.0) (Math|Vector|MakeVector _x _y 0.0)))))))
      (else
        (Variables|Default|SetdividerTempVar (Class|KismetMathLibrary|DegAcos (Math|Vector|DotProduct (Variables|Default|GetXvector) (Math|Vector|Normalize (- (Math|Vector|MakeVector (.X (Math|Vector|BreakVector (Transformation|GetActorLocation _array_element))) (.Y (Math|Vector|BreakVector (Transformation|GetActorLocation _array_element))) 0.0) (Math|Vector|MakeVector _x _y 0.0))))))))
    (if (== (/ (Variables|Default|GetdividerTempVar) (/ 360 _returnvalue_3)) _returnvalue_3)
      (LocalVariables|SetRoboIndex 0)
      (else
        (LocalVariables|SetRoboIndex (/ (Variables|Default|GetdividerTempVar) (/ 360 _returnvalue_3)))))
    (Default|AddWaypoint (Utilities|Array|Get(acopy) _robos (LocalVariables|GetRoboIndex)) _array_element)))

(fn MakeColors
  (Utilities|Array|Add (Variables|Default|Getcolors) (Math|Conversions|ToColor(LinearColor) (Class|KismetMathLibrary|LinearColorRed)))
  (Utilities|Array|Add (Variables|Default|Getcolors) (Math|Conversions|ToColor(LinearColor) (Class|KismetMathLibrary|LinearColorBlue)))
  (Utilities|Array|Add (Variables|Default|Getcolors) (Math|Conversions|ToColor(LinearColor) (Class|KismetMathLibrary|LinearColorGreen)))
  (Utilities|Array|Add (Variables|Default|Getcolors) (Math|Conversions|ToColor(LinearColor) (Class|KismetMathLibrary|LinearColorYellow)))
  (Utilities|Array|Add (Variables|Default|Getcolors) (Math|Conversions|ToColor(LinearColor) (Class|KismetMathLibrary|LinearColorWhite)))
  (Utilities|Array|Add (Variables|Default|Getcolors) (Math|Conversions|ToColor(LinearColor) (Math|Color|MakeColor 128.0 0.0 128.0)))
  (Utilities|Array|Add (Variables|Default|Getcolors) (Math|Conversions|ToColor(LinearColor) (Math|Color|MakeColor 0.0 255.0 255.0)))
  (Utilities|Array|Add (Variables|Default|Getcolors) (Math|Conversions|ToColor(LinearColor) (Math|Color|MakeColor 255.0 0.0 255.0)))
  (Utilities|Array|Add (Variables|Default|Getcolors) (Math|Conversions|ToColor(LinearColor) (Math|Color|MakeColor 255.0 192.0 203.0)))
  (Utilities|Array|Add (Variables|Default|Getcolors) (Math|Conversions|ToColor(LinearColor) (Math|Color|MakeColor 165.0 42.0 42.0))))