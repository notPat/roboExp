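; Explore-mode player controller for a lidar scanning level, turning input into signals and fly-speed changes.
; B, Tab and K fire the build map, show lidar and render-point-cloud-in-new-level signals for listeners outside this Blueprint.
; Mouse wheel steps a clamped speed into the pawn's FloatingPawnMovement.
; BeginPlay caches visible actors without the Lidar tag, but the FlipFlop that would toggle their visibility is disconnected.
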(event EventBeginPlay
  (bind _outactors (Actor|GetAllActorsOfClass "/Script/Engine.Actor"))
  (for _array_element _outactors
    (if (not (Actor|ActorHasTag _array_element "Lidar"))
      (if (not (Variables|/Script/Engine.Actor|GetbHidden _array_element))
        (Utilities|Array|Add (Variables|Default|GetToggeledHideActors) _array_element)))))

(event EventTick
  (params (DeltaSeconds :type Float%20%28single-precision%29)))

(event Input|MouseEvents|MouseWheelAxis
  (params (AxisValue :type Float%20%28single-precision%29))
  (if (!= AxisValue 0.0)
    (Variables|Default|SetCurrentSpeed (Math|Float|Clamp(Float) (+ (Variables|Default|GetCurrentSpeed) (* (Variables|Default|GetSpeedStep) AxisValue)) (Variables|Default|GetMinSpeed) (Variables|Default|GetMaxSpeed)))
    (bind _asfloating_pawn_movement (Utilities|Casting|CastToFloatingPawnMovement (Pawn|GetMovementComponent (Game|Player|GetPlayerPawn 0))))
    (Variables|/Script/Engine.FloatingPawnMovement|SetMaxSpeed _asfloating_pawn_movement (Variables|Default|GetCurrentSpeed))))

(event Input|KeyboardEvents|B
  (params (Key :type Key%20Structure :default "None"))
  (:Pressed
    (Default|CallBuildMapSig)))

(event Input|KeyboardEvents|Tab
  (params (Key :type Key%20Structure :default "None"))
  (:Pressed
    (Default|CallShowLidarSig)))

(event Input|KeyboardEvents|K
  (params (Key :type Key%20Structure :default "None"))
  (:Pressed
    (Default|CallRenderPointCloudinNewLevelSig)))

(fn ConstructionScript)