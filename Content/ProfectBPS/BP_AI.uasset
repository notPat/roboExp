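; Patrolling AI actor that endlessly travels a looping list of waypoints.
; On BeginPlay it starts its Scanner and moves itself to a nearby point projected onto the navmesh.
; Explore uses AIMoveTo toward the current waypoint, then advances and wraps the index on success or failure before calling itself again.
; AddWaypoint appends entries to the route.
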(event Custom|Explore
  (AI|AIMoveTo self "0, 0, 0" (Utilities|Array|Get(acopy) (Variables|Default|GetWaypoints) (Variables|Default|GetWaypointIndex)) 1e+01 false
    (:OnSuccess
      _)
    (:OnFail
      _))
  (bind _result (Math|Integer|IncrementInt (Variables|Default|GetWaypointIndex))
    (:%20%20
      (if (>= _result (Utilities|Array|Length (Variables|Default|GetWaypoints)))
        (Variables|Default|SetWaypointIndex 0))
      (CallFunction|Explore))))

(event EventBeginPlay
  (Default|BeginScanning (Variables|Default|GetScanner))
  (Transformation|SetActorLocation (.ProjectedLocation (AI|Navigation|ProjectPointtoNavigation (Transformation|GetActorLocation) 0 0 "2000.000000,200.000000,500.000000")) false false)
  (CallFunction|Explore))

(event EventTick
  (params (DeltaSeconds :type Float%20%28single-precision%29)))

(event Collision|EventActorBeginOverlap
  (params (OtherActor :type Actor%20Object%20Reference)))

(fn ConstructionScript)

(fn AddWaypoint
  (params (wp :type BP%20Waypont%20Object%20Reference))
  (Utilities|Array|Add (Variables|Default|GetWaypoints) wp))