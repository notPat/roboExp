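; BP_AI is a scanning agent that picks waypoints toward the sparsest sector of its Scanner's point grid.
; StartUp begins scanning, snaps the actor to the navmesh, and labels and colors its waypoints.
; NextWaypoint decodes the lowest-count "X_Y_Z" grid key, returning it as look-at and a nearby waypoint as destination, with visit tracking and random fallback.
; Waypoint sorting and sequential patrol logic are unconnected.
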(event Custom|StartUp
  (bind _signiturecolor (Variables|Default|GetSignitureColor))
  (Default|BeginScanning (Variables|Default|GetScanner))
  (Transformation|SetActorLocation (.ProjectedLocation (AI|Navigation|ProjectPointtoNavigation (Transformation|GetActorLocation) 0 0 "200.000000,200.000000,1000.000000")) false true)
  (for _array_element (Variables|Default|GetWaypoints)
    (Default|SetTextRender _array_element (Utilities|String|Append (Utilities|GetObjectName self) "->" (Utilities|GetObjectName _array_element)) _signiturecolor)
    (Variables|/Game/ProfectBPS/LidarCloudGen/Scanner.Scanner_C|SetSigColor (Variables|Default|GetScanner) _signiturecolor)))

(event EventBeginPlay)

(event EventTick
  (params (DeltaSeconds :type Float%20%28single-precision%29)))

(event Collision|EventActorBeginOverlap
  (params (OtherActor :type Actor%20Object%20Reference)))

(fn ConstructionScript)

(fn AddWaypoint
  (params (wp :type BP%20Waypoint%20Object%20Reference))
  (Utilities|Array|Add (Variables|Default|GetWaypoints) wp))

(fn NextWaypoint
  (bind _waypoints (Variables|Default|GetWaypoints))
  (bind _waypoints_2 (Variables|Default|GetWaypoints))
  (bind _scanner (Variables|Default|GetScanner))
  (bind _waypoints_3 (Variables|Default|GetWaypoints))
  (bind _returnvalue (Utilities|Array|Length _waypoints))
  (bind _gridpointcount (Variables|/Game/ProfectBPS/LidarCloudGen/Scanner.Scanner_C|GetGridPointCount _scanner))
  (bind (_key _value) (Utilities|Map|GetKeyValueByIndex _gridpointcount 0))
  (bind _returnvalue_2 (Math|Random|RandomInteger _returnvalue))
  (bind _output (Utilities|Array|Get(acopy) _waypoints_2 _returnvalue_2))
  (if (== (Utilities|Array|Length (Variables|Default|GetVisitedWPs)) (Utilities|Array|Length (Variables|Default|GetWaypoints)))
    (Utilities|Array|Clear (Variables|Default|GetVisitedWPs)))
  (Variables|Default|SetlowestDensitySector _key)
  (Variables|Default|SetlowestDensityAmount _value)
  (bind (_keypin _valuepin) (Utilities|Map|ForEachLoop(Map) _gridpointcount)
    (:then
      (if (< _valuepin (Variables|Default|GetlowestDensityAmount))
        (Variables|Default|SetlowestDensitySector _keypin)
        (Variables|Default|SetlowestDensityAmount _valuepin)))
    (:CompletedPin
      (bind _output_get (Variables|Default|SetLowestDistWP (Utilities|Array|Get(acopy) _waypoints_3)))
      (Variables|Default|SetlowestDist (Math|Vector|VectorLength (- (Transformation|GetActorLocation _output_get) (* (Math|Vector|MakeVector (Math|Conversions|ToFloat(Integer) (.LeftS (Utilities|String|Split (Variables|Default|GetlowestDensitySector) "_"))) (Math|Conversions|ToFloat(Integer) (.LeftS (Utilities|String|Split (.RightS (Utilities|String|Split (Variables|Default|GetlowestDensitySector) "_")) "_"))) (Math|Conversions|ToFloat(Integer) (.RightS (Utilities|String|Split (.RightS (Utilities|String|Split (Variables|Default|GetlowestDensitySector) "_")) "_")))) "1000.000000,1000.000000,1000.000000"))))
      (for _array_element _waypoints_3
        (if (and (not (Utilities|Array|ContainsItem (Variables|Default|GetVisitedWPs) _array_element)) (< (Math|Vector|VectorLength (- (* (Math|Vector|MakeVector (Math|Conversions|ToFloat(Integer) (.LeftS (Utilities|String|Split (Variables|Default|GetlowestDensitySector) "_"))) (Math|Conversions|ToFloat(Integer) (.LeftS (Utilities|String|Split (.RightS (Utilities|String|Split (Variables|Default|GetlowestDensitySector) "_")) "_"))) (Math|Conversions|ToFloat(Integer) (.RightS (Utilities|String|Split (.RightS (Utilities|String|Split (Variables|Default|GetlowestDensitySector) "_")) "_")))) "1000.000000,1000.000000,1000.000000") (Transformation|GetActorLocation _array_element))) (Variables|Default|GetlowestDist)))
          (Variables|Default|SetLowestDistWP _array_element)
          (Variables|Default|SetlowestDist (Math|Vector|VectorLength (- (* (Math|Vector|MakeVector (Math|Conversions|ToFloat(Integer) (.LeftS (Utilities|String|Split (Variables|Default|GetlowestDensitySector) "_"))) (Math|Conversions|ToFloat(Integer) (.LeftS (Utilities|String|Split (.RightS (Utilities|String|Split (Variables|Default|GetlowestDensitySector) "_")) "_"))) (Math|Conversions|ToFloat(Integer) (.RightS (Utilities|String|Split (.RightS (Utilities|String|Split (Variables|Default|GetlowestDensitySector) "_")) "_")))) "1000.000000,1000.000000,1000.000000") (Transformation|GetActorLocation _array_element))))))
      (if (Utilities|Array|ContainsItem (Variables|Default|GetVisitedWPs) (Variables|Default|GetLowestDistWP))
        (Utilities|FlowControl|ForLoopwithBreak 0 _returnvalue :!label _label
          (:LoopBody
            (if (Utilities|Array|ContainsItem (Variables|Default|GetVisitedWPs) _output)
              (Variables|Default|SetLowestDistWP _output)
              (goto _label Break)))
          (:Completed
            (Utilities|Array|Add (Variables|Default|GetVisitedWPs) (Variables|Default|GetLowestDistWP) :!label _label_2)
            (return (Transformation|GetActorLocation (Variables|Default|GetLowestDistWP)) (* (Math|Vector|MakeVector (Math|Conversions|ToFloat(Integer) (.LeftS (Utilities|String|Split (Variables|Default|GetlowestDensitySector) "_"))) (Math|Conversions|ToFloat(Integer) (.LeftS (Utilities|String|Split (.RightS (Utilities|String|Split (Variables|Default|GetlowestDensitySector) "_")) "_"))) (Math|Conversions|ToFloat(Integer) (.RightS (Utilities|String|Split (.RightS (Utilities|String|Split (Variables|Default|GetlowestDensitySector) "_")) "_")))) "1000.000000,1000.000000,1000.000000"))))
        (else
          (goto _label_2))))))