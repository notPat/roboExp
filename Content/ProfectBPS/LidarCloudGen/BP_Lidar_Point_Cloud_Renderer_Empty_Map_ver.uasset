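; Actor that displays the lidar point cloud stored in BP_ExploreInstance, with exploration stats and file export.
; On BeginPlay it sets the cloud, counts points per grid cell in a string-keyed map, and fills a hidden WBP_LidarStats widget with density, time, distance and point totals.
; Player controller signal toggles widget and mouse input; widget signal exports points to XYZ under Saved/Exports.
; The binding for opening VehicleBasic never runs.
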(event Custom|ShowLidarSig_Event
  (bind _returnvalue (Game|GetPlayerController 0))
  (Utilities|FlowControl|FlipFlop
    (:A
      (Variables|/Script/UMG.Widget|SetVisibility (Variables|Default|GetLidarStatsWidged) "Visible")
      (Variables|/Script/Engine.PlayerController|SetbShowMouseCursor _returnvalue true)
      (Input|SetInputModeGameandUI _returnvalue 0 "DoNotLock" false false))
    (:B
      (Variables|/Script/UMG.Widget|SetVisibility (Variables|Default|GetLidarStatsWidged) "Hidden")
      (Variables|/Script/Engine.PlayerController|SetbShowMouseCursor _returnvalue false)
      (Input|SetInputModeGameOnly _returnvalue false))))

(event Custom|ExportLidarCloudToFile_Event
  (bind _newparam (Default|GetFilename (Variables|Default|GetLidarStatsWidged)))
  (bind _returnvalue (Class|UtilityFunctions|ExportXYZ (Utilities|String|Append (Class|KismetSystemLibrary|GetProjectSavedDirectory) "Exports/" _newparam ".xyz") (Variables|/Game/ProfectBPS/BP_ExploreInstance.BP_ExploreInstance_C|Getpoints (stale EventBeginPlay _asbp_explore_instance)) 0.0))
  (Development|PrintString (Utilities|String|Append (Class|KismetSystemLibrary|GetProjectSavedDirectory) "Exports/" _newparam ".xyz") (not _returnvalue) true "(R=0.000000,G=0.660000,B=1.000000,A=1.000000)" 2e+01))

(event Custom|RenderPointCloudInNewLevelSig_Event
  (Development|PrintString "Called")
  (Game|OpenLevel(byName) "VehicleBasic" false))

(event Collision|EventActorBeginOverlap
  (params (OtherActor :type Actor%20Object%20Reference)))

(event EventTick
  (params (DeltaSeconds :type Float%20%28single-precision%29)))

(event EventBeginPlay
  (bind _gridstep (Variables|Default|GetGridStep))
  (bind _gridpointcount (Variables|Default|GetGridPointCount))
  (bind _returnvalue (UserInterface|CreateWidget "/Game/ProfectBPS/Menu/WBP_LidarStats.WBP_LidarStats_C"))
  (UserInterface|Viewport|AddtoViewport _returnvalue 0)
  (Variables|/Script/UMG.Widget|SetVisibility _returnvalue "Hidden")
  (Variables|Default|SetLidarStatsWidged _returnvalue)
  (bind _asbp_explore_player_controler (Utilities|Casting|CastToBP_ExplorePlayerControler (Game|GetPlayerController 0)))
  (EventDispatchers|AssignShowLidarSig _asbp_explore_player_controler (delegate Custom|ShowLidarSig_Event))
  (bind _asbp_explore_instance (Utilities|Casting|CastToBP_ExploreInstance (Game|GetGameInstance)))
  (Variables|Default|SetExploration%20Time (Variables|/Game/ProfectBPS/BP_ExploreInstance.BP_ExploreInstance_C|GetExplorationTime _asbp_explore_instance))
  (Variables|Default|SetExploration%20Distance (Variables|/Game/ProfectBPS/BP_ExploreInstance.BP_ExploreInstance_C|GetExplorationDistance _asbp_explore_instance))
  (Class|LidarPointCloudComponent|SetPointCloud (Variables|Default|GetLidarPointCloud) (Variables|/Game/ProfectBPS/BP_ExploreInstance.BP_ExploreInstance_C|GetPointCloud _asbp_explore_instance))
  (bind _asbp_explore_player_controler_2 (Utilities|Casting|CastToBP_ExplorePlayerControler (Game|GetPlayerController 0)))
  (EventDispatchers|AssignExportLidarCloudtoFile (Variables|Default|GetLidarStatsWidged) (delegate Custom|ExportLidarCloudToFile_Event))
  (Variables|Default|SetPointAmount (Utilities|Array|Length (Variables|/Game/ProfectBPS/BP_ExploreInstance.BP_ExploreInstance_C|Getpoints _asbp_explore_instance)))
  (for _array_element (Variables|/Game/ProfectBPS/BP_ExploreInstance.BP_ExploreInstance_C|Getpoints _asbp_explore_instance)
    (if (Utilities|Map|Contains (Variables|Default|GetGridPointCount) (Utilities|String|Append (Utilities|String|ToString(Integer) (Class|KismetMathLibrary|ToInt64(Float) (/ (.X (Math|Vector|BreakVector (.Location (Utilities|Struct|BreakLidarPointCloudPoint _array_element)))) _gridstep))) " " (Utilities|String|ToString(Integer) (Class|KismetMathLibrary|ToInt64(Float) (/ (.Y (Math|Vector|BreakVector (.Location (Utilities|Struct|BreakLidarPointCloudPoint _array_element)))) _gridstep))) " " (Utilities|String|ToString(Integer) (Class|KismetMathLibrary|ToInt64(Float) (/ (.Z (Math|Vector|BreakVector (.Location (Utilities|Struct|BreakLidarPointCloudPoint _array_element)))) _gridstep)))))
      (bind _result (Math|Integer|IncrementInt (.Value (Utilities|Map|Find _gridpointcount (Utilities|String|Append (Utilities|String|ToString(Integer) (Class|KismetMathLibrary|ToInt64(Float) (/ (.X (Math|Vector|BreakVector (.Location (Utilities|Struct|BreakLidarPointCloudPoint _array_element)))) _gridstep))) " " (Utilities|String|ToString(Integer) (Class|KismetMathLibrary|ToInt64(Float) (/ (.Y (Math|Vector|BreakVector (.Location (Utilities|Struct|BreakLidarPointCloudPoint _array_element)))) _gridstep))) " " (Utilities|String|ToString(Integer) (Class|KismetMathLibrary|ToInt64(Float) (/ (.Z (Math|Vector|BreakVector (.Location (Utilities|Struct|BreakLidarPointCloudPoint _array_element)))) _gridstep)))))))
        (:%20%20
          (Utilities|Map|Add _gridpointcount (Utilities|String|Append (Utilities|String|ToString(Integer) (Class|KismetMathLibrary|ToInt64(Float) (/ (.X (Math|Vector|BreakVector (.Location (Utilities|Struct|BreakLidarPointCloudPoint _array_element)))) _gridstep))) " " (Utilities|String|ToString(Integer) (Class|KismetMathLibrary|ToInt64(Float) (/ (.Y (Math|Vector|BreakVector (.Location (Utilities|Struct|BreakLidarPointCloudPoint _array_element)))) _gridstep))) " " (Utilities|String|ToString(Integer) (Class|KismetMathLibrary|ToInt64(Float) (/ (.Z (Math|Vector|BreakVector (.Location (Utilities|Struct|BreakLidarPointCloudPoint _array_element)))) _gridstep)))) _result)))
      (else
        (Utilities|Map|Add (Variables|Default|GetGridPointCount) (Utilities|String|Append (Utilities|String|ToString(Integer) (Class|KismetMathLibrary|ToInt64(Float) (/ (.X (Math|Vector|BreakVector (.Location (Utilities|Struct|BreakLidarPointCloudPoint _array_element)))) _gridstep))) " " (Utilities|String|ToString(Integer) (Class|KismetMathLibrary|ToInt64(Float) (/ (.Y (Math|Vector|BreakVector (.Location (Utilities|Struct|BreakLidarPointCloudPoint _array_element)))) _gridstep))) " " (Utilities|String|ToString(Integer) (Class|KismetMathLibrary|ToInt64(Float) (/ (.Z (Math|Vector|BreakVector (.Location (Utilities|Struct|BreakLidarPointCloudPoint _array_element)))) _gridstep)))) 1))))
  (bind (_keypin _valuepin) (Utilities|Map|ForEachLoop(Map) (Variables|Default|GetGridPointCount))
    (:then
      (Variables|Default|SetGridDensity (Utilities|String|Append (Variables|Default|GetGridDensity) (Utilities|String|Append _keypin ": " (Utilities|String|ToString(Integer) _valuepin)) "{0}")))
    (:CompletedPin
      (Rendering|Components|TextRender|SetText (Variables|/Game/ProfectBPS/Menu/WBP_LidarStats.WBP_LidarStats_C|GetDensityGridList (Variables|Default|GetLidarStatsWidged)) (Utilities|Text|FormatText (Utilities|Text|ToText(String) (Variables|Default|GetGridDensity)) (Variables|Default|GetNewLine)))
      (Rendering|Components|TextRender|SetText (Variables|/Game/ProfectBPS/Menu/WBP_LidarStats.WBP_LidarStats_C|GetGerneralInfo (Variables|Default|GetLidarStatsWidged)) (Utilities|Text|FormatText (Utilities|Text|ToText(String) (Utilities|String|Append (Utilities|String|MakeLiteralString "Time of simulation : ") (Utilities|String|ToString(Float) (Variables|Default|GetExploration%20Time)) "{0}" "Amount of Points scanned : " (Utilities|String|ToString(Integer) (Variables|Default|GetPointAmount)) "{0}" "Exploration distance: " (Utilities|String|ToString(Integer) (Variables|Default|GetExploration%20Distance)))) (Variables|Default|GetNewLine))))))

(fn ConstructionScript)